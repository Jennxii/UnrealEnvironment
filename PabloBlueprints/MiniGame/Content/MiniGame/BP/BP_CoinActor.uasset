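; Collectible mini-game coin that spins, changes denomination and, on overlap, adds its value to BP_FH_Tutrial_Character before destroying itself.
; SetCoinState swaps the mesh and value for Coin1, Coin2 and Coin5, though Coin5's value assignment is disconnected, leaving the previous value.
; BeginPlay cycles all three states through an endless Delay loop.
; A one-shot timer and the E key also drive a FlipFlop between Coin1 and Coin5.
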(event OnComponentBeginOverlap(SM_Coin_1)
  (params (OverlappedComponent :type Primitive%20Component%20Object%20Reference) (OtherActor :type Actor%20Object%20Reference) (OtherComp :type Primitive%20Component%20Object%20Reference) (OtherBodyIndex :type Integer) (bFromSweep :type Boolean) (SweepResult :type Hit%20Result%20Structure%20%28by%20ref%29))
  ;[0.15 0.15 0.15 0.5] add coins to character
  (bind _asbp_fh_tutrial_character (Utilities|Casting|CastToBP_FH_Tutrial_Character OtherActor))
  (Default|AddCoin _asbp_fh_tutrial_character (Variables|Default|GetCoinValue))
  (Actor|DestroyActor))

(event Custom|SwitchCoinState_timer
  (Utilities|FlowControl|FlipFlop
    (:A
      (CallFunction|SetCoinState "NewEnumerator0"))
    (:B
      (CallFunction|SetCoinState "NewEnumerator2"))))

(event EventBeginPlay
  (Utilities|Time|SetTimerbyEvent (delegate Custom|SwitchCoinState_timer) 5.0)
  (CallFunction|SetCoinState "NewEnumerator0" :!label _label)
  (Utilities|FlowControl|Delay 5.0)
  (CallFunction|SetCoinState "NewEnumerator1")
  (Utilities|FlowControl|Delay 5.0)
  (CallFunction|SetCoinState "NewEnumerator2")
  (Utilities|FlowControl|Delay 5.0)
  (goto _label))

(event EventTick
  (params (DeltaSeconds :type Float%20%28single-precision%29))
  (Transformation|AddActorLocalRotation (Math|Rotator|MakeRotator 0.0 0.0 (* (Variables|Setup|GetRotationSpeed) DeltaSeconds)) false false))

(event Input|KeyboardEvents|E
  (params (Key :type Key%20Structure :default "None"))
  (:Pressed
    (Utilities|FlowControl|FlipFlop
      (:A
        (CallFunction|SetCoinState "NewEnumerator0"))
      (:B
        (CallFunction|SetCoinState "NewEnumerator2")))))

(fn ConstructionScript
  (CallFunction|SetCoinState "NewEnumerator0"))

(fn NewFunction)

(fn SetCoinState
  (params (NewState :type Enum_CoinState%20Enum :default "NewEnumerator0"))
  (switch Utilities|FlowControl|Switch|SwitchonEnum_CoinState NewState
    (:NewEnumerator0
      (Components|StaticMesh|SetStaticMesh (Variables|Default|GetSM_Coin_1) "/Game/Import/SM_Coin_1.SM_Coin_1")
      (Variables|Default|SetCoinValue 1))
    (:NewEnumerator1
      (Components|StaticMesh|SetStaticMesh (Variables|Default|GetSM_Coin_1) "/Game/Import/SM_Coin_2.SM_Coin_2")
      (Variables|Default|SetCoinValue 2))
    (:NewEnumerator2
      (Components|StaticMesh|SetStaticMesh (Variables|Default|GetSM_Coin_1) "/Game/Import/SM_Coin_5.SM_Coin_5"))))