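; BP_CoinSpawner is a minigame actor that spawns a row of BP_CoinActor coins along world X from its own transform, spaced by Distance.
; SpawnCoins destroys the coins tracked in CoinActorsArray, then spawns and stores a new set, each with a randomly picked CoinStateSetup.
; BeginPlay repeats this on a looping five-second delay, and the SpawninEditor event exposes the same spawn as a separate trigger.
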(event Custom|Spawn%20in%20Editor
  (CallFunction|SpawnCoins))

(event EventBeginPlay
  (CallFunction|SpawnCoins :!label _label)
  (Utilities|FlowControl|Delay 5.0)
  (goto _label))

(fn ConstructionScript)

(fn SpawnCoins
  (bind _returnvalue (Transformation|GetActorTransform))
  ;[0.15 0.15 0.15 0.5] delete array items
  (for _array_element (Variables|Default|GetCoinActorsArray)
    (Utilities|IsValid _array_element
      (:Is%20Valid
        (Actor|DestroyActor _array_element))))
  (Utilities|Array|Clear (Variables|Default|GetCoinActorsArray))
  ;[0.15 0.15 0.15 0.5] Spawn Coins
  (for _index (range 0 (Variables|Default|GetNumberOfCoins))
    (bind _returnvalue_2 (Game|SpawnActorfromClass "/Game/MiniGame/BP/BP_CoinActor.BP_CoinActor_C" (Math|Transform|MakeTransform (Math|Vector|MakeVector (+ (.x (.location _returnvalue)) (* _index (Variables|Default|GetDistance))) (.y (.location _returnvalue)) (.z (.location _returnvalue))) (.rotation _returnvalue) (.scale _returnvalue)) "Undefined" "MultiplyWithRoot" 0 60 (.OutItem (Utilities|Array|Random (Utilities|Array|MakeArray "NewEnumerator0" "NewEnumerator1" "NewEnumerator2"))) 0))
    ;[0.15 0.15 0.15 0.5] add coins to array
    (Utilities|Array|Add (Variables|Default|GetCoinActorsArray) _returnvalue_2)))